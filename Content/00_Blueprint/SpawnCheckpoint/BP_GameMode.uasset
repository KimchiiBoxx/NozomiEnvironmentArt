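; Game mode that respawns the player at the last checkpoint reached, or at a PlayerStart if none is set.
; On login it stores the controller and restarts the player, binding to the pawn's destroyed event on each restart to trigger the next respawn.
; UpdateSpawnLocation sets the checkpoint that the FindPlayerStart override returns.
; Only one controller reference is kept, so respawning tracks just the latest player to join.
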(event `self.K2_PostLogin`
  (params (NewPlayer :type "PlayerController Object Reference"))
  (bind _output_get (set `self.ControllerRef` NewPlayer))
  (`self.RestartPlayer` _output_get))

(event `self.K2_OnRestartPlayer`
  (params (NewPlayer :type "Controller Object Reference"))
  ;[1 1 1] When pawn is destroy - start event
  (add `self.OnDestroyed` (`Controller.K2_GetPawn` NewPlayer) (delegate `PawnDied`)))

(event `PawnDied` :!signature `self.OnDestroyed`
  (params (DestroyedActor :type "Actor Object Reference"))
  (`self.RestartPlayer` (`self.ControllerRef`)))

(event `/Game/00_Blueprint/SpawnCheckpoint/BPI_UpdateSpawnLocation.UpdateSpawnLocation`
  (params (NewLocation :type "Actor Object Reference"))
  (set `self.SpawnLocation` NewLocation))

(fn `FindPlayerStart`
  (params (Player :type "Controller Object Reference") (IncomingName :type String))
  (returns (ReturnValue :type "Actor Object Reference"))
  ;[1 1 1] if pass checkpoint spawn there, otherwise spawn at start
  (bind _spawnlocation (`self.SpawnLocation`)
    (:`then`
      (return _spawnlocation))
    (:`else`
      (bind _returnvalue (`GameplayStatics.GetActorOfClass` "/Script/Engine.PlayerStart"))
      (return _returnvalue))))

(fn `UserConstructionScript`)