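; BP_PickUpItem_7 is a pickup actor for the Origami Crane item that reveals a letter when collected.
; Its PickUp event prints a received message, destroys the actor, then adds the BPW_06_Letter widget to the viewport and flags it as open.
; The Construction Script applies the ItemMeshToPlace variable to the static mesh component.
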(event `/Game/00_Storytelling/BPI_Interaction.PickUp`
  ;[1 1 1] After press E = destroy Item and print Information
  (`KismetSystemLibrary.PrintString` "You received an Origami Crane.")
  (`self.K2_DestroyActor`)
  ;[1 1 1] When Item destroyed = show Letter
  (`/Engine/EditorBlueprintResources/StandardMacros.IsValid` (`self.Widget`)
    (:`Is Valid`
      _)
    (:`Is Not Valid`
      (`|CreateWidget` "/Game/00_Storytelling/BPW_06_Letter.BPW_06_Letter_C")
      (set `self.Widget` null)))
  (`UserWidget.AddToViewport` (`self.Widget`) 0)
  (set `self.WidgetIsOpen` true))

(fn `UserConstructionScript`
  (`StaticMeshComponent.SetStaticMesh` (`self.StaticMesh`) (`self.ItemMeshToPlace`)))