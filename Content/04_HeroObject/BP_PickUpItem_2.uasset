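; Pickup item actor that gives the player an Origami Crane and opens a letter widget.
; An interaction sign turns toward the camera every tick and is visible while BP_SadakoCharacter overlaps the trigger collider.
; The PickUp event prints a message, destroys the actor, then creates the BPW_02_Letter widget if needed, adds it to the viewport and flags it as open.
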(event `/Game/00_Storytelling/BPI_Interaction.PickUp`
  ;[1 1 1] After press E = destroy Item and print Information
  (`KismetSystemLibrary.PrintString` "You received an Origami Crane.")
  (`self.K2_DestroyActor`)
  ;[1 1 1] When Item destroyed = show Letter
  (`/Engine/EditorBlueprintResources/StandardMacros.IsValid` (`self.Widget`)
    (:`Is Valid`
      _)
    (:`Is Not Valid`
      (bind _returnvalue (`|CreateWidget` "/Game/00_Storytelling/BPW_02_Letter.BPW_02_Letter_C"))
      (set `self.Widget` _returnvalue)))
  (`UserWidget.AddToViewport` (`self.Widget`) 0)
  (set `self.WidgetIsOpen` true))

(event `self.ReceiveTick`
  (params (DeltaSeconds :type "Float (single-precision)"))
  ;[1 1 1] Direction of Interaction Sign
  (`SceneComponent.K2_SetWorldRotation` (`self.InteractionSign`) (`KismetMathLibrary.FindLookAtRotation` (`SceneComponent.K2_GetComponentLocation` (`self.InteractionSign`)) (`SceneComponent.K2_GetComponentLocation` (`PlayerCameraManager.TransformComponent` (`GameplayStatics.GetPlayerCameraManager` 0)))) false false))

(event `self.TriggerCollider.OnComponentBeginOverlap`
  (params (OverlappedComponent :type "PrimitiveComponent Object Reference") (OtherActor :type "Actor Object Reference") (OtherComp :type "PrimitiveComponent Object Reference") (OtherBodyIndex :type Integer) (bFromSweep :type Boolean) (SweepResult :type "HitResult Structure (by ref)"))
  ;[1 1 1] Show Interaction Sign
  (cast `/Game/03_Character/Sadako/Blueprint/BP_SadakoCharacter` OtherActor)
  (`SceneComponent.SetVisibility` (`self.InteractionSign`) true false))

(event `self.TriggerCollider.OnComponentEndOverlap`
  (params (OverlappedComponent :type "PrimitiveComponent Object Reference") (OtherActor :type "Actor Object Reference") (OtherComp :type "PrimitiveComponent Object Reference") (OtherBodyIndex :type Integer))
  ;[1 1 1] Show Interaction Sign
  (cast `/Game/03_Character/Sadako/Blueprint/BP_SadakoCharacter` OtherActor)
  (`SceneComponent.SetVisibility` (`self.InteractionSign`) false false))

(fn `UserConstructionScript`
  (`AddComponent|NODE_AddStaticMeshComponent-0`))